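; A spinning actor that, on its first hit, sends a named analytics event to Mixpanel.
; It builds a JSON event array with the logged-in user ID, UTC Unix timestamp and unique insert ID as properties.
; The array is POSTed to Mixpanel's import endpoint with a Basic authorization header built from the encoded project token.
; The response handler prints the result and destroys the actor once the body converts to a string.
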(event Custom|OnMixpanelEventSent
  (params (ResponseStatus :type EM2_HttpResponseStatus%20Enum :default "OK") (ResponseCode :type Integer) (ResponseHeaders :type M2%20Http%20Response%20Headers%20Structure%20%28by%20ref%29) (ResponseBody :type M2%20Http%20Response%20Content%20Structure%20%28by%20ref%29) (CorrelationId :type Guid%20Structure%20%28by%20ref%29))
  (bind _returnvalue (Class|M2HttpUtilsFunctionLibrary|GetHttpResponseStringContent ResponseBody)
    (:Success
      (Development|PrintString (Utilities|String|Append "Status: " (Utilities|String|EnumtoString ResponseStatus) " Code: " (Utilities|String|ToString(Integer) ResponseCode) " Body: " _returnvalue) true true "(R=1.000000,G=0.000000,B=0.007519,A=1.000000)" 1e+02)
      (Actor|DestroyActor))
    (:Invalid
      (Development|PrintString "Invalid string conversion" true true "(R=0.000000,G=0.660000,B=1.000000,A=1.000000)" 1e+02))))

(event Custom|SendMixPanelData
  (bind _jsonobjectwrapper (Utilities|Struct|MakeJsonObjectWrapper))
  (bind _returnvalue (Class|M2PlayerProfileSubsystem|GetPlayerProfileSubsystem))
  (bind _returnvalue_2 (Class|M2JsonFunctionLibrary|CreateJsonValueString (Class|M2PlayerProfileSubsystem|GetLoggedinUserIdString _returnvalue)))
  (Class|M2JsonFunctionLibrary|SetJsonObjectFieldValue _jsonobjectwrapper "distinct_id" _returnvalue_2)
  (bind _returnvalue_3 (Class|M2JsonFunctionLibrary|CreateJsonValueNumber (Math|Conversions|ToFloat(Integer) (Class|M2DateFunctionLibrary|GetUnixTimestampfromDateTime (Math|DateTime|UTCNow)))))
  (Class|M2JsonFunctionLibrary|SetJsonObjectFieldValue _jsonobjectwrapper "time" _returnvalue_3)
  (bind _returnvalue_4 (Class|M2JsonFunctionLibrary|CreateJsonValueString (Guid|ToString(Guid) (Guid|NewGuid))))
  (Class|M2JsonFunctionLibrary|SetJsonObjectFieldValue _jsonobjectwrapper "$insert_id" _returnvalue_4)
  (bind _outjsonobject (Class|M2JsonFunctionLibrary|MakeJsonObjectfromStruct (Utilities|Struct|MakeMixpanelEvent (Utilities|String|MakeLiteralString (Variables|Default|GetEventName)))))
  (bind _returnvalue_5 (Class|M2JsonFunctionLibrary|CreateJsonValueObject _jsonobjectwrapper))
  (Class|M2JsonFunctionLibrary|SetJsonObjectFieldValue _outjsonobject "properties" _returnvalue_5)
  (bind _returnvalue_6 (Class|M2JsonFunctionLibrary|CreateJsonValueObjectArray (Utilities|Array|MakeArray _outjsonobject)))
  (bind _returnvalue_7 (Class|M2HttpUtilsFunctionLibrary|CreateJsonValueContent _returnvalue_6)
    (:Success
      (bind _returnvalue_8 (Class|M2HttpUtilsFunctionLibrary|CreateHttpRequestHeaders (Utilities|Map|MakeMap "Authorization" (Utilities|String|Append "Basic " (Variables|Default|GetEncodedProjectToken)))))
      (Class|M2HttpUtilsFunctionLibrary|SendHttpRequestBP :Url "https://api.mixpanel.com/import" :Verb "POST" :RequestHeaders _returnvalue_8 :RequestBody _returnvalue_7 :OnComplete (EventDispatchers|CreateEvent :!event Custom|OnMixpanelEventSent)
        (:InvalidUrl
          _)
        (:UrlBlocked
          _)
        (:InvalidVerb
          _)
        (:InvalidContent
          _)
        (:InvalidHeaders
          _)
        (:FailedToSend
          _))
      (Development|PrintString "Something Went Wrong with Sending Http Request! " true true "(R=0.000000,G=0.660000,B=1.000000,A=1.000000)" 1e+01))
    (:Invalid
      (Development|PrintString "Failed Creating Mixpanel Json Content"))))

(event EventBeginPlay)

(event EventTick
  (params (DeltaSeconds :type Float%20%28single-precision%29))
  (|CallParentFunction DeltaSeconds)
  (Transformation|AddActorLocalRotation (Math|Rotator|MakeRotator 0.0 0.0 (* DeltaSeconds (Variables|Default|GetRotation))) false false))

(event Collision|EventHit
  (params (MyComp :type Primitive%20Component%20Object%20Reference) (Other :type Actor%20Object%20Reference) (OtherComp :type Primitive%20Component%20Object%20Reference) (bSelfMoved :type Boolean) (HitLocation :type Vector :default "0, 0, 0") (HitNormal :type Vector :default "0, 0, 0") (NormalImpulse :type Vector :default "0, 0, 0") (Hit :type Hit%20Result%20Structure%20%28by%20ref%29))
  (|CallParentFunction MyComp Other OtherComp bSelfMoved HitLocation HitNormal NormalImpulse Hit)
  (if (not (Variables|Default|GetSendingReq))
    (Variables|Default|SetSendingReq true)
    (Development|PrintString "Now Sending Mixpanel Event")
    (CallFunction|SendMixPanelData)))

(fn ConstructionScript)